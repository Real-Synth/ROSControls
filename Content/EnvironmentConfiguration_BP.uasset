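; Environment configuration actor that applies scene and simulation settings on construction and every tick.
; Wood-versus-concrete sleeper and foliage toggles are written as scalar parameters to the MeshSwap_MPC material parameter collection.
; It also pushes the simulation time step to the ROSIntegration game instance's fixed update interval and dirt mask intensity to the BP_ScenarioManager, caching both references.
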(event EventBeginPlay)

(event Collision|EventActorBeginOverlap
  (params (OtherActor :type Actor%20Object%20Reference)))

(event EventTick
  (params (DeltaSeconds :type Float%20%28single-precision%29))
  (CallFunction|Update))

(fn ConstructionScript
  (CallFunction|Update))

(fn UpdateMPC
  (bind _woodsleepers (Variables|Default|GetWoodSleepers))
  (bind _returnvalue (Math|Float|SelectFloat 1.0 0.0 _woodsleepers))
  (Utilities|FlowControl|Sequence
    (:then_0
      (Rendering|Material|SetScalarParameterValue "/Game/Environment/Railway/Materials/MeshSwap_MPC.MeshSwap_MPC" "WoodSleepers" _returnvalue :!class /Script/Engine.KismetMaterialLibrary)
      (Rendering|Material|SetScalarParameterValue "/Game/Environment/Railway/Materials/MeshSwap_MPC.MeshSwap_MPC" "ConcreteSleepers" (- 1.0 _returnvalue) :!class /Script/Engine.KismetMaterialLibrary))
    (:then_1
      (Rendering|Material|SetScalarParameterValue "/Game/Environment/Railway/Materials/MeshSwap_MPC.MeshSwap_MPC" "Foliage" (Math|Float|SelectFloat 1.0 0.0 (Variables|Default|GetFoliage)) :!class /Script/Engine.KismetMaterialLibrary))))

(fn Update
  (Utilities|FlowControl|Sequence
    (:then_0
      (CallFunction|UpdateMPC))
    (:then_1
      (Variables|Default|GetSimulationInstance
        (:then
          _)
        (:else
          (bind _asrosintegration_game_instance (Utilities|Casting|CastToROSIntegrationGameInstance (Game|GetGameInstance)))
          (Variables|Default|SetSimulationInstance _asrosintegration_game_instance)))
      (Variables|/Script/ROSIntegration.ROSIntegrationGameInstance|SetFixedUpdateInterval (Variables|Default|GetSimulationInstance) (Variables|Default|GetSimulationTimeStep)))
    (:then_2
      (Variables|Default|GetScenarioManager
        (:then
          _)
        (:else
          (bind _outactors (Actor|GetAllActorsOfClass "/Game/FunctionalAssets/BP_ScenarioManager.BP_ScenarioManager_C"))
          (Variables|Default|SetScenarioManager (Utilities|Array|Get(acopy) _outactors))))
      (Variables|/Game/FunctionalAssets/BP_ScenarioManager.BP_ScenarioManager_C|SetDirtMaskIntensity (Variables|Default|GetScenarioManager) (Variables|Default|GetDirtMaskIntensity)))))